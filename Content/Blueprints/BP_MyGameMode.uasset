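; BP_MyGameMode is a game mode that plays an opening cutscene, then hands control to the player.
; On BeginPlay it creates and plays the LS_OpeningCutscene level sequence and binds to its finished event.
; When the sequence ends, it spawns BP_ThirdPersonCharacter at the found PlayerStart, with debug prints of that start, and has player controller 0 possess it.
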(event Custom|OnCutsceneFinished
  ;[0.15 0.15 0.15 0.5] Opening Cutscene to Player handover
  (bind _returnvalue (Actor|GetActorOfClass "/Script/Engine.PlayerStart"))
  (Development|PrintString (Utilities|GetDisplayName _returnvalue))
  (Development|PrintString (Utilities|String|ToString(Transform) (Transformation|GetActorTransform _returnvalue)))
  (bind _returnvalue_2 (Game|SpawnActorfromClass "/Game/ThirdPerson/Blueprints/BP_ThirdPersonCharacter.BP_ThirdPersonCharacter_C" (Transformation|GetActorTransform _returnvalue) "AdjustIfPossibleButAlwaysSpawn" "MultiplyWithRoot" 0 0))
  (Pawn|Possess (Game|GetPlayerController 0) _returnvalue_2))

(event EventBeginPlay
  ;[0.15 0.15 0.15 0.5] Opening Cutscene to Player handover
  (bind _returnvalue (Sequencer|Player|CreateLevelSequencePlayer "/Game/Cutscenes/Opening/LS_OpeningCutscene.LS_OpeningCutscene"))
  (bind _output_get (Variables|Default|SetOpeningCutscenePlayer _returnvalue))
  (Sequencer|Player|Play _returnvalue :!class /Script/MovieScene.MovieSceneSequencePlayer)
  (EventDispatchers|BindEventtoOnFinished _output_get (delegate Custom|OnCutsceneFinished)))

(event EventTick
  (params (DeltaSeconds :type Float%20%28single-precision%29)))

(fn ConstructionScript)