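; BP_NPC is an interactable NPC that plays a configurable idle animation and can speak a voice line.
; A trigger overlap registers the NPC as the third-person character's CurrentNPC, shows an interaction prompt widget and enables input on the NPC.
; Leaving the trigger clears that reference, removes the prompt and disables input.
; PlayVoiceLine_Event plays the voice line at the NPC's location under a concurrency setting, with no caller in this Blueprint.
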(event OnComponentBeginOverlap(Trigger)
  (params (OverlappedComponent :type Primitive%20Component%20Object%20Reference) (OtherActor :type Actor%20Object%20Reference) (OtherComp :type Primitive%20Component%20Object%20Reference) (OtherBodyIndex :type Integer) (bFromSweep :type Boolean) (SweepResult :type Hit%20Result%20Structure%20%28by%20ref%29))
  ;[0.15 0.15 0.15 0.5] Approach
  (Development|PrintString "overlap fired")
  (bind _asbp_third_person_character (Utilities|Casting|CastToBP_ThirdPersonCharacter OtherActor))
  (Development|PrintString "Cast Succeeded - Player Detected!")
  (Variables|/Game/ThirdPerson/Blueprints/BP_ThirdPersonCharacter.BP_ThirdPersonCharacter_C|SetCurrentNPC _asbp_third_person_character self)
  (bind _returnvalue (UserInterface|CreateWidget "/Game/UI/WBP_InteractionPrompt.WBP_InteractionPrompt_C" (Game|GetPlayerController 0)))
  (bind _output_get (Variables|Default|SetInteractionWidget _returnvalue))
  (UserInterface|Viewport|AddtoViewport _output_get 0)
  (Input|EnableInput self (Game|GetPlayerController 0))
  (Development|PrintString "INPUT ENABLED FOR NPC"))

(event OnComponentEndOverlap(Trigger)
  (params (OverlappedComponent :type Primitive%20Component%20Object%20Reference) (OtherActor :type Actor%20Object%20Reference) (OtherComp :type Primitive%20Component%20Object%20Reference) (OtherBodyIndex :type Integer))
  (bind _interactionwidget (Variables|Default|GetInteractionWidget))
  ;[0.15 0.15 0.15 0.5] End overlap
  (Development|PrintString "Cast ended, player left")
  (bind _asbp_third_person_character (Utilities|Casting|CastToBP_ThirdPersonCharacter OtherActor))
  (Variables|/Game/ThirdPerson/Blueprints/BP_ThirdPersonCharacter.BP_ThirdPersonCharacter_C|SetCurrentNPC _asbp_third_person_character 0)
  (Utilities|IsValid _interactionwidget
    (:Is%20Valid
      (Widget|RemovefromParent _interactionwidget)
      (Input|DisableInput self (Game|GetPlayerController 0)))))

(event Custom|PlayVoiceLine_Event
  (Audio|PlaySoundatLocation (Variables|Default|GetVoiceLine) (Transformation|GetActorLocation) "0, 0, 0" 1.0 1.0 0.0 0 "/Game/Audio/SC_VoiceLines.SC_VoiceLines" 0 0))

(event EventBeginPlay)

(event Collision|EventActorBeginOverlap
  (params (OtherActor :type Actor%20Object%20Reference)))

(event EventTick
  (params (DeltaSeconds :type Float%20%28single-precision%29))
  ;[0.15 0.15 0.15 0.5] Approach
)

(fn ConstructionScript
  (Components|Animation|OverrideAnimationData (Variables|Character|GetMesh) (Variables|Default|GetIdleAnimation) true true 0.0 1.0))